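; BP_TV is an interactable living-room television that the player can switch on and off.
; On Interact it runs the parent logic, then a FlipFlop alternates between the two states.
; On applies a TV light function material to a point light, raises its intensity and plays ambience audio; off clears the material, zeroes the light and stops the sound.
; Each toggle updates the interaction prompt, and ambience is stopped at BeginPlay.
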(event EventBeginPlay
  (Audio|Components|Audio|Stop (Variables|Default|GetSC_TVAmbiance)))

(event EventInteract
  (params (Player :type Player%20Character%20Object%20Reference))
  (bind _sc_tvambiance (Variables|Default|GetSC_TVAmbiance))
  (bind _pointlight (Variables|Default|GetPointLight))
  (|CallParentFunction Player)
  (Utilities|FlowControl|FlipFlop
    (:A
      (Rendering|Components|Light|SetLightFunctionMaterial _pointlight "/Game/Assets/Marketplace/LivingRoom/Materials/M_TVLight.M_TVLight")
      (Rendering|Components|Light|SetIntensity _pointlight 5e+03)
      (Audio|Components|Audio|Play _sc_tvambiance 0.0)
      (Variables|Default|SetInteractionPrompt "Press [Space] to turn TV off."))
    (:B
      (Rendering|Components|Light|SetLightFunctionMaterial _pointlight 0)
      (Rendering|Components|Light|SetIntensity _pointlight 0.0)
      (Audio|Components|Audio|Stop _sc_tvambiance)
      (Variables|Default|SetInteractionPrompt "Press [Space] to turn TV on."))))

(fn ConstructionScript)